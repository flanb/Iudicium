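; BP_Vase is a breakable vase that plays a shattering sound when its Chaos geometry collection breaks.
; The break event passes through a DoOnce, so only the first fracture triggers audio.
; Nested random rolls pick one of three break sounds, weighted toward the first.
; The sound is positioned at GetWorldOriginLocation, the world origin, rather than at the vase's own location.
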(event OnChaosBreakEvent(GeometryCollectionComponent)
  (params (BreakEvent :type Chaos%20Break%20Event%20Structure%20%28by%20ref%29))
  (bind _returnvalue (Class|GameplayStatics|GetWorldOriginLocation))
  (bind _returnvalue_2 (Math|Random|RandomInteger 2))
  (bind _returnvalue_3 (Math|Conversions|ToVector(Float) _returnvalue))
  (Utilities|FlowControl|DoOnce false
    (:Completed
      (if (== _returnvalue_2 0)
        (Audio|PlaySoundatLocation "/Game/sound/vases/VASE_BREAKING.VASE_BREAKING" _returnvalue_3 "0, 0, 0" 1.0 1.0 0.0 0 0 0 0)
        (elif (== _returnvalue_2 1)
          (Audio|PlaySoundatLocation "/Game/sound/vases/VASE_BREAKING2.VASE_BREAKING2" _returnvalue_3 "0, 0, 0" 1.0 1.0 0.0 0 0 0 0)
          (else
            (Audio|PlaySoundatLocation "/Game/sound/vases/VASE_BREAKING3.VASE_BREAKING3" _returnvalue_3 "0, 0, 0" 1.0 1.0 0.0 0 0 0 0)))))))

(event EventBeginPlay)

(event Collision|EventActorBeginOverlap
  (params (OtherActor :type Actor%20Object%20Reference)))

(event EventTick
  (params (DeltaSeconds :type Float%20%28single-precision%29)))

(fn ConstructionScript)