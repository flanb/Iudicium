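; BP_DoorReincarnation is a door that swings open when approached and sends the game to an ending level.
; Overlapping the Open volume plays a timeline that drives the mesh's yaw and the rect light's intensity together.
; Overlapping the TPLevel volume loads L_EndScreen if IsVoid is set, otherwise L_End; neither overlap filters the overlapping actor.
; The construction script writes TextArea to the text render as the door's label.
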(event OnComponentBeginOverlap(Open)
  (params (OverlappedComponent :type Primitive%20Component%20Object%20Reference) (OtherActor :type Actor%20Object%20Reference) (OtherComp :type Primitive%20Component%20Object%20Reference) (OtherBodyIndex :type Integer) (bFromSweep :type Boolean) (SweepResult :type Hit%20Result%20Structure%20%28by%20ref%29))
  (bind (_direction _anglez _lumen) (Timeline|Timeline Play)
    (:Update
      (Transformation|SetRelativeRotation (Variables|Default|GetStaticMesh) (Math|Rotator|MakeRotator 0.0 0.0 _anglez) false true)
      (Rendering|Components|Light|SetIntensity (Variables|Default|GetRectLight) _lumen))))

(event OnComponentBeginOverlap(TPLevel)
  (params (OverlappedComponent :type Primitive%20Component%20Object%20Reference) (OtherActor :type Actor%20Object%20Reference) (OtherComp :type Primitive%20Component%20Object%20Reference) (OtherBodyIndex :type Integer) (bFromSweep :type Boolean) (SweepResult :type Hit%20Result%20Structure%20%28by%20ref%29))
  (if (Variables|Default|GetIsVoid)
    (Game|OpenLevel(byObjectReference) "/Game/Maps/L_EndScreen.L_EndScreen")
    (else
      (Game|OpenLevel(byObjectReference) "/Game/Maps/L_End.L_End"))))

(event EventBeginPlay)

(event Collision|EventActorBeginOverlap
  (params (OtherActor :type Actor%20Object%20Reference)))

(event EventTick
  (params (DeltaSeconds :type Float%20%28single-precision%29)))

(fn ConstructionScript
  (Rendering|Components|TextRender|SetText (Variables|Default|GetTextRender) (Variables|Default|GetTextArea)))