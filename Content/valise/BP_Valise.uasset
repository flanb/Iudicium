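; Suitcase that unlocks and opens itself when a BP_Key actor first overlaps its trigger box.
; The key is moved and attached to KeyParent, which then plays a scripted sequence: turn back and forth, slide sideways, turn again.
; MoveComponentTo drives the key motion, with Delays spacing the steps.
; Timelines then pitch the valise mesh open and rescale the key before destroying it.
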(event OnComponentBeginOverlap(Box)
  (params (OverlappedComponent :type Primitive%20Component%20Object%20Reference) (OtherActor :type Actor%20Object%20Reference) (OtherComp :type Primitive%20Component%20Object%20Reference) (OtherBodyIndex :type Integer) (bFromSweep :type Boolean) (SweepResult :type Hit%20Result%20Structure%20%28by%20ref%29))
  (bind _keyparent (Variables|Default|GetkeyParent))
  (Utilities|Casting|CastToBP_Key OtherActor)
  (Utilities|FlowControl|DoOnce false
    (:Completed
      (Variables|Default|SetOther%20Actor OtherActor)
      (bind _output_get (Variables|Default|SetOther%20Comp OtherComp))
      (Components|MoveComponentTo _output_get (Transformation|GetWorldLocation _keyparent) (Transformation|GetWorldRotation _keyparent) true true 5.0 true)
      (Transformation|AttachComponentToComponent _output_get (Variables|Default|GetkeyParent) "None" "SnapToTarget" "SnapToTarget" "KeepWorld" true)
      (Physics|SetSimulatePhysics (Variables|Default|GetOther%20Comp) false)
      (CallFunction|TurnKey)
      (Utilities|FlowControl|Delay 2.0)
      (CallFunction|MovetoNext)
      (Utilities|FlowControl|Delay 2.0)
      (CallFunction|TurnKey)
      (Utilities|FlowControl|Delay 0.2)
      (CallFunction|Open)
      (bind _newtrack_0 (Timeline|Timeline_0 Play)
        (:Update
          (Transformation|SetWorldScale3D (Variables|Default|GetOther%20Comp) (Math|Conversions|ToVector(Float) _newtrack_0)))
        (:Finished
          (Actor|DestroyActor (Variables|Default|GetOther%20Actor)))))))

(event Custom|Open
  (bind _valise_fe3_004 (Variables|Default|Getvalise_Fe3_004))
  (bind _returnvalue (Transformation|GetWorldRotation _valise_fe3_004))
  (bind _newtrack_0 (Timeline|Timeline Play)
    (:Update
      (Transformation|SetWorldRotation _valise_fe3_004 (Math|Rotator|MakeRotator (.roll _returnvalue) _newtrack_0 (.yaw _returnvalue)) false false))))

(event Custom|TurnKey
  (bind _keyparent (Variables|Default|GetkeyParent))
  (bind _returnvalue (Transformation|GetRelativeTransform _keyparent))
  (Components|MoveComponentTo _keyparent (.location _returnvalue) (Math|Rotator|MakeRotator (+ (.roll (.rotation _returnvalue)) 45.0) (.pitch (.rotation _returnvalue)) (.yaw (.rotation _returnvalue))) true true 1.0 true)
  (Components|MoveComponentTo _keyparent (.location _returnvalue) (Math|Rotator|MakeRotator (- (.roll (.rotation _returnvalue)) 45.0) (.pitch (.rotation _returnvalue)) (.yaw (.rotation _returnvalue))) true true 1.0 true))

(event Custom|Move%20to%20next
  (bind _keyparent (Variables|Default|GetkeyParent))
  (bind _returnvalue (Transformation|GetRelativeTransform _keyparent))
  (Components|MoveComponentTo _keyparent (+ (.location _returnvalue) "0.000000,-40.000000,0.000000") (.rotation _returnvalue) true true 2.0 true))

(event EventBeginPlay)

(event Collision|EventActorBeginOverlap
  (params (OtherActor :type Actor%20Object%20Reference)))

(event EventTick
  (params (DeltaSeconds :type Float%20%28single-precision%29)))

(fn ConstructionScript)